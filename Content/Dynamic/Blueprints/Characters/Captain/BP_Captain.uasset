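; BP_Captain is the playable side-view character, handling Enhanced Input movement, jumping, attacks and sword throwing.
; Actions are gated by CanAct, with ground, air and throw animation overrides toggling IsAttaking, and velocity flipping controller yaw for facing.
; GainAbility records unlocks that enable double jump or throwing, while a separate SpawnSword event creates the projectile.
; On defeat it prints a loss message and restarts through GM_Action after a delay.
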(event `self.ReceiveBeginPlay`
  (`parent.ReceiveBeginPlay`)
  (bind _asplayer_controller (cast `PlayerController` (`self.GetController`)))
  (`EnhancedInputSubsystemInterface.AddMappingContext` (pcsubsystem `EnhancedInputLocalPlayerSubsystem` _asplayer_controller) "/Game/Dynamic/Inputs/IMC_Action.IMC_Action" 0 (struct))
  (add `self.Defeated` (delegate `OnDefeated`)))

(event `OnDefeated`
  (bind _asgm_action (cast `/Game/Dynamic/Blueprints/GM_Action` (`GameplayStatics.GetGameMode`)))
  (`KismetSystemLibrary.PrintString` "OYUNU KAYBETTİNİZ!!!")
  (`KismetSystemLibrary.Delay` 1.5)
  (`/Game/Dynamic/Blueprints/GM_Action.RestartGame` _asgm_action))

(event `self.ReceiveTick`
  (params (DeltaSeconds :type "Float (single-precision)"))
  (`parent.ReceiveTick` 0.0)
  (`self.UpdatedControllerRotation`))

(event `EnhancedInput|/Game/Dynamic/Inputs/Actions/IA_Jump`
  (params (ActionValue :type Boolean) (ElapsedSeconds :type "Float (double-precision)") (TriggeredSeconds :type "Float (double-precision)") (InputAction :type "InputAction Object Reference" :default "/Game/Dynamic/Inputs/Actions/IA_Jump.IA_Jump"))
  (:`Started`
    (if (`self.CanAct`)
      (`self.Jump`)))
  (:`Completed`
    (`self.StopJumping`)))

(event `EnhancedInput|/Game/Dynamic/Inputs/Actions/IA_Move`
  (params (ActionValue :type "Vector2D Structure") (ElapsedSeconds :type "Float (double-precision)") (TriggeredSeconds :type "Float (double-precision)") (InputAction :type "InputAction Object Reference" :default "/Game/Dynamic/Inputs/Actions/IA_Move.IA_Move"))
  (bind (_x _y) (`KismetMathLibrary.BreakVector2D` ActionValue))
  (:`Triggered`
    (if (`self.CanAct`)
      (`self.AddMovementInput` (1.0 0.0 0.0) _x)
      (if (not (`self.LockTo2D`))
        (`self.AddMovementInput` (0.0 -1.0 0.0) _y)))))

(event `EnhancedInput|/Game/Dynamic/Inputs/Actions/IA_Attack`
  (params (ActionValue :type Boolean) (ElapsedSeconds :type "Float (double-precision)") (TriggeredSeconds :type "Float (double-precision)") (InputAction :type "InputAction Object Reference" :default "/Game/Dynamic/Inputs/Actions/IA_Attack.IA_Attack"))
  (:`Started`
    (if (`self.CanAct`)
      (if (`NavMovementComponent.IsMovingOnGround` (`self.CharacterMovement`))
        (`PaperZDPlaySlotOverrideAction.PlayAnimationOverrideWithCallbacks` (`self.AnimInstance`) "/Game/Dynamic/Blueprints/Characters/Captain/AnimSequences/Attack.Attack"
          (:`then`
            (set `self.IsAttaking` true))
          (:`OnCompleted`
            (set `self.IsAttaking` false :!label _label))
          (:`OnCancelled`
            (goto _label)))
        (else
          (`PaperZDPlaySlotOverrideAction.PlayAnimationOverrideWithCallbacks` (`self.AnimInstance`) "/Game/Dynamic/Blueprints/Characters/Captain/AnimSequences/AirAttack.AirAttack"
            (:`then`
              (set `self.IsAttaking` true))
            (:`OnCompleted`
              (set `self.IsAttaking` false :!label _label_2))
            (:`OnCancelled`
              (goto _label_2))))))))

(event `EnhancedInput|/Game/Dynamic/Inputs/Actions/IA_Throw`
  (params (ActionValue :type Boolean) (ElapsedSeconds :type "Float (double-precision)") (TriggeredSeconds :type "Float (double-precision)") (InputAction :type "InputAction Object Reference" :default "/Game/Dynamic/Inputs/Actions/IA_Throw.IA_Throw"))
  (:`Started`
    (if (and (`KismetArrayLibrary.Array_Contains` (`self.UnluckedAbilityes`) "NewEnumerator1") (`self.CanAct`))
      (`PaperZDPlaySlotOverrideAction.PlayAnimationOverrideWithCallbacks` (`self.GetAnimInstance`) "/Game/Dynamic/Blueprints/Characters/Captain/AnimSequences/Throw.Throw"
        (:`then`
          (set `self.IsAttaking` true))
        (:`OnCompleted`
          (set `self.IsAttaking` false :!label _label_3))
        (:`OnCancelled`
          (goto _label_3))))))

(event `SpawnSword`
  (bind _returnvalue (`|SpawnActorFromClass` "/Game/Dynamic/Blueprints/BP_Sword.BP_Sword_C" (`KismetMathLibrary.MakeTransform` (`SceneComponent.K2_GetComponentLocation` (`self.ThrowPos`)) (`self.K2_GetActorRotation`)) "AlwaysSpawn" "MultiplyWithRoot" null null))
  (set `self.ActiveSword` _returnvalue))

(fn `GainAbility`
  (params (AbilityType :type "/Game/Dynamic/Blueprints/Enums/E_Abilities Enum (by ref)"))
  (`KismetArrayLibrary.Array_AddUnique` (`self.UnluckedAbilityes`) AbilityType)
  (switch `/Game/Dynamic/Blueprints/Enums/E_Abilities` (`local.AbilityType`)
    (:`NewEnumerator0`
      (set `self.JumpMaxCount` 2))))

(fn `UpdatedControllerRotation`
  (bind _returnvalue (`self.GetController`))
  (bind _returnvalue_2 (`self.GetController`))
  (bind _velocity_x (`KismetMathLibrary.BreakVector` (`MovementComponent.Velocity` (`self.CharacterMovement`))))
  (`/Engine/EditorBlueprintResources/StandardMacros.CompareFloat` _velocity_x
    (:`>`
      (`/Engine/EditorBlueprintResources/StandardMacros.IsValid` _returnvalue_2
        (:`Is Valid`
          (`Controller.SetControlRotation` _returnvalue_2 (`KismetMathLibrary.MakeRotator` 0.0)))))
    (:`<`
      (`/Engine/EditorBlueprintResources/StandardMacros.IsValid` _returnvalue
        (:`Is Valid`
          (`Controller.SetControlRotation` _returnvalue (`KismetMathLibrary.MakeRotator` 0.0 0.0 180.0)))))))

(fn `UserConstructionScript`
  (`parent.UserConstructionScript`))