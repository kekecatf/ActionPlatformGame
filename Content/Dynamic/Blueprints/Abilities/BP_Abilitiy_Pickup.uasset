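; Ability pickup actor that grants the player captain an ability and triggers shark spawns when collected.
; When a BP_Captain overlaps the PlayerCheck component, it passes its AbilityType to the captain's GainAbility and prints a Turkish debug message with the ability name.
; It then calls SpawnShark on every entry in its Spawners array and destroys itself.
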(event `self.PlayerCheck.OnComponentBeginOverlap`
  (params (OverlappedComponent :type "PrimitiveComponent Object Reference") (OtherActor :type "Actor Object Reference") (OtherComp :type "PrimitiveComponent Object Reference") (OtherBodyIndex :type Integer) (bFromSweep :type Boolean) (SweepResult :type "HitResult Structure (by ref)"))
  (bind _asbp_captain (cast `/Game/Dynamic/Blueprints/Characters/Captain/BP_Captain` OtherActor))
  (`/Game/Dynamic/Blueprints/Characters/Captain/BP_Captain.GainAbility` _asbp_captain (`self.AbilityType`))
  (`KismetSystemLibrary.PrintString` "Yetenegini Kazandin")
  (`KismetSystemLibrary.PrintString` (`|GetEnumeratorNameAsString` (`self.AbilityType`)))
  (for _array_element (`self.Spawners`)
    (`/Game/Dynamic/Blueprints/BP_Spawner.SpawnShark` _array_element))
  (`self.K2_DestroyActor`))

(fn `UserConstructionScript`)